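; BP_Brick is a brick for an Arkanoid-style game that gives visual and audio feedback when damaged.
; Its DamageFeedback event reads BrickLife and, while life remains, sets the ArkanoidTile material from a Materials map keyed by that value.
; At zero or below, it spawns an explosion particle at the brick's transform and plays a 2D blast sound.
; The graph itself neither changes BrickLife nor destroys the actor.
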(event EventDamageFeedback
  (if (> (Variables|Default|GetBrickLife) 0)
    (Rendering|Material|SetMaterial (Variables|Default|GetArkanoid_Tile) 0 (.Value (Utilities|Map|Find (Variables|Default|GetMaterials) (Variables|Default|GetBrickLife))))
    (else
      (Effects|SpawnEmitteratLocation "/Game/Visual/PS_BrickExplode.PS_BrickExplode" (Transformation|GetActorLocation) (Transformation|GetActorRotation))
      (Audio|PlaySound2D "/Game/Sounds/Blast_10.Blast_10" 1.0 1.0 0.0 0 0))))

(fn ConstructionScript)